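; Moving platform actor that travels along its Arrow component's forward direction.
; On BeginPlay it stores its start location, sets the 이동그래프 timeline's play rate from PlayTime, waits RateTime, then plays it.
; Each timeline update offsets the start location along the arrow by the 이동값 curve value times MoveScale, without sweep.
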(event `self.ReceiveBeginPlay`
  (set `self.StartPos` (`self.K2_GetActorLocation`))
  (`TimelineComponent.SetPlayRate` (`self.이동 그래프`) (`self.PlayTime`))
  (`KismetSystemLibrary.Delay` (`self.RateTime`))
  (bind (_direction `_이동값`) (`Timeline|이동 그래프`)
    (:`Update`
      (`self.K2_SetActorLocation` (+ (`self.StartPos`) (* (`SceneComponent.GetForwardVector` (`self.Arrow`)) (* `_이동값` (`self.MoveScale`))))))))

(fn `UserConstructionScript`)